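; Player camera manager that provides a free-moving camera with a set rotation and adjustable height, detached from any pawn.
; CameraMove offsets the given location in one of eight directions, clamping X to the area's Left/Right and Y to Back/Forward.
; UpdateHeight scales input by HeightSpeed and clamps height between a floor and the area's limit.
; BlueprintUpdateCamera outputs the stored position, height, rotation and default FOV when the target is BP_PlayerController.
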(event `self.ReceiveBeginPlay`
  (set `self.PlayerCameraLocation` (0.0 0.0 0.0)))

(event `self.ReceiveTick`
  (params (DeltaSeconds :type "Float (single-precision)")))

(fn `BlueprintUpdateCamera`
  (params (CameraTarget :type "Actor Object Reference"))
  (returns (NewCameraLocation :type "Vector Structure") (NewCameraRotation :type "Rotator Structure") (NewCameraFOV :type "Float (single-precision)") (ReturnValue :type Boolean))
  (bind _asbp_player_controller (cast `/Game/Nav/BP_PlayerController` CameraTarget))
  (return (`KismetMathLibrary.MakeVector` (.x (`self.PlayerCameraLocation`)) (.y (`self.PlayerCameraLocation`)) (`self.CameraHeight`)) (`self.Camera Rotation`) (`PlayerCameraManager.DefaultFOV` (`PlayerController.PlayerCameraManager` _asbp_player_controller)) true))

(fn `CameraMove`
  (params (Directional :type "/Game/Datas/E_CameraMovementDirectional Enum" :default "NewEnumerator0") (CameraLocation :type "Vector Structure"))
  (locals (MoveValue :type "Vector Structure"))
  (bind (_left _right _forward _back) (break `/Game/Datas/CameraMoveArea` (`self.MovementArea`)))
  (`|ExecutionSequence`
    (:`then_0`
      (switch `/Game/Datas/E_CameraMovementDirectional` (`local.Directional`)
        (:`NewEnumerator0`
          (set `local.MoveValue` (`KismetMathLibrary.MakeVector` 0.0 (* (`self.MovementSpeed`) -1.0))))
        (:`NewEnumerator1`
          (set `local.MoveValue` (`KismetMathLibrary.MakeVector` 0.0 (* (`self.MovementSpeed`) 1.0))))
        (:`NewEnumerator2`
          (set `local.MoveValue` (`KismetMathLibrary.MakeVector` (* (`self.MovementSpeed`) 1.0))))
        (:`NewEnumerator3`
          (set `local.MoveValue` (`KismetMathLibrary.MakeVector` (* (`self.MovementSpeed`) -1.0))))
        (:`NewEnumerator4`
          (set `local.MoveValue` (`KismetMathLibrary.MakeVector` (* (`self.MovementSpeed`) 1.0) (* (`self.MovementSpeed`) -1.0))))
        (:`NewEnumerator5`
          (set `local.MoveValue` (`KismetMathLibrary.MakeVector` (* (`self.MovementSpeed`) 1.0) (* (`self.MovementSpeed`) 1.0))))
        (:`NewEnumerator6`
          (set `local.MoveValue` (`KismetMathLibrary.MakeVector` (* (`self.MovementSpeed`) -1.0) (* (`self.MovementSpeed`) -1.0))))
        (:`NewEnumerator7`
          (set `local.MoveValue` (`KismetMathLibrary.MakeVector` (* (`self.MovementSpeed`) -1.0) (* (`self.MovementSpeed`) 1.0))))))
    (:`then_1`
      (set `self.PlayerCameraLocation` (`KismetMathLibrary.MakeVector` (`KismetMathLibrary.FClamp` (.x (+ CameraLocation (`local.MoveValue`))) _left _right) (`KismetMathLibrary.FClamp` (.y (+ CameraLocation (`local.MoveValue`))) _back _forward))))))

(fn `UpdateHeight`
  (params (Value :type "Float (double-precision)"))
  (set `self.CameraHeight` (`KismetMathLibrary.FClamp` (+ (`self.CameraHeight`) (* Value (`self.HeightSpeed`))) 50.0 (`.Height_10_E42663F349B55141ADFC12A5EF2A42FB` (break `/Game/Datas/CameraMoveArea` (`self.MovementArea`))))))

(fn `UserConstructionScript`)