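; Player controller that drives an edge-scrolling camera with mouse-wheel height control.
; BeginPlay sizes the screen-edge bands as a ratio of the DPI-scaled viewport.
; Each Tick, when InValidArea finds the cursor in a band, JudgeMovementDirectional classifies it into one of eight edge or corner directions for BP_PlayerCameraManager's CameraMove.
; Mouse wheel input goes to the camera manager's UpdateHeight.
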(event `self.ReceiveBeginPlay`
  (bind _returnvalue (`WidgetLayoutLibrary.GetViewportScale`))
  (bind _validratio (`self.ValidRatio`))
  (bind (_x _y) (`KismetMathLibrary.BreakVector2D` (`self.ScreenSize`)))
  (set `self.ScreenSize` (/ (`WidgetLayoutLibrary.GetViewportSize`) (`KismetMathLibrary.MakeVector2D` _returnvalue _returnvalue)))
  (set `self.ValidBorder_X` (* _x _validratio))
  (set `self.ValidBorder_Y` (* _y _validratio)))

(event `self.ReceiveTick`
  (params (DeltaSeconds :type "Float (single-precision)"))
  (bind (_locationx _locationy) (`WidgetLayoutLibrary.GetMousePositionScaledByDPI` self))
  (bind _returnvalue (`KismetMathLibrary.MakeVector2D` _locationx _locationy))
  (bind _asbp_player_camera_manager (cast `/Game/Nav/BP_PlayerCameraManager` (`self.PlayerCameraManager`)))
  (if (`self.InValidArea` _returnvalue)
    (`/Game/Nav/BP_PlayerCameraManager.CameraMove` _asbp_player_camera_manager (`self.JudgeMovementDirectional` _returnvalue) (`PlayerCameraManager.GetCameraLocation` _asbp_player_camera_manager))))

(event `InputAxisKey|MouseWheelAxis`
  (params (AxisValue :type "Float (single-precision)"))
  (bind _asbp_player_camera_manager (cast `/Game/Nav/BP_PlayerCameraManager` (`self.PlayerCameraManager`)))
  (`/Game/Nav/BP_PlayerCameraManager.UpdateHeight` _asbp_player_camera_manager AxisValue))

(fn `InValidArea`
  (params (`Mouse Location` :type "Vector2D Structure"))
  (returns (InInvalidArea :type Boolean))
  (bind (_x _y) (`KismetMathLibrary.BreakVector2D` `Mouse Location`))
  (bind _validborder_x (`self.ValidBorder_X`))
  (bind _validborder_y (`self.ValidBorder_Y`))
  (bind (_x_2 _y_2) (`KismetMathLibrary.BreakVector2D` (`self.ScreenSize`)))
  (return (not (and (`KismetMathLibrary.InRange_FloatFloat` _x _validborder_x (- _x_2 _validborder_x)) (`KismetMathLibrary.InRange_FloatFloat` _y _validborder_y (- _y_2 _validborder_y))))))

(fn `JudgeMovementDirectional`
  (params (`Mouse Location` :type "Vector2D Structure"))
  (returns (NewParam :type "/Game/Datas/E_CameraMovementDirectional Enum"))
  (locals (LeftRight :type "/Game/Datas/LeftRight Enum") (ForwardBackward :type "/Game/Datas/ForwardBackward Enum"))
  (bind _validborder_y (`self.ValidBorder_Y`))
  (bind _validborder_x (`self.ValidBorder_X`))
  (`|ExecutionSequence`
    (:`then_0`
      (`|ExecutionSequence`
        (:`then_0`
          (if (`KismetMathLibrary.InRange_FloatFloat` (`KismetMathLibrary.BreakVector2D` (`local.Mouse Location`)) _validborder_x (- (`KismetMathLibrary.BreakVector2D` (`self.ScreenSize`)) _validborder_x))
            (set `local.LeftRight` "NewEnumerator2")
            (elif (`KismetMathLibrary.InRange_FloatFloat` (`KismetMathLibrary.BreakVector2D` (`local.Mouse Location`)) 0.0 (`self.ValidBorder_X`))
              (set `local.LeftRight` "NewEnumerator0")
              (else
                (set `local.LeftRight` "NewEnumerator1")))))
        (:`then_1`
          (if (`KismetMathLibrary.InRange_FloatFloat` (`.Y` (`KismetMathLibrary.BreakVector2D` (`local.Mouse Location`))) _validborder_y (- (`.Y` (`KismetMathLibrary.BreakVector2D` (`self.ScreenSize`))) _validborder_y))
            (set `local.ForwardBackward` "NewEnumerator2")
            (elif (`KismetMathLibrary.InRange_FloatFloat` (`.Y` (`KismetMathLibrary.BreakVector2D` (`local.Mouse Location`))) 0.0 (`self.ValidBorder_Y`))
              (set `local.ForwardBackward` "NewEnumerator0")
              (else
                (set `local.ForwardBackward` "NewEnumerator1")))))))
    (:`then_1`
      (if (`|EnumEquality` (`local.LeftRight`) "NewEnumerator2")
        (if (`|EnumEquality` (`local.ForwardBackward`) "NewEnumerator0")
          (return "NewEnumerator2")
          (else
            (return "NewEnumerator3")))
        (elif (`|EnumEquality` (`local.ForwardBackward`) "NewEnumerator2")
          (if (`|EnumEquality` (`local.LeftRight`) "NewEnumerator0")
            (return "NewEnumerator0")
            (else
              (return "NewEnumerator1")))
          (elif (and (`|EnumEquality` (`local.ForwardBackward`) "NewEnumerator0") (`|EnumEquality` (`local.LeftRight`) "NewEnumerator0"))
            (return "NewEnumerator4")
            (elif (and (`|EnumEquality` (`local.ForwardBackward`) "NewEnumerator0") (`|EnumEquality` (`local.LeftRight`) "NewEnumerator1"))
              (return "NewEnumerator5")
              (elif (and (`|EnumEquality` (`local.ForwardBackward`) "NewEnumerator1") (`|EnumEquality` (`local.LeftRight`) "NewEnumerator0"))
                (return "NewEnumerator6")
                (else
                  (return "NewEnumerator7"))))))))))

(fn `UserConstructionScript`)